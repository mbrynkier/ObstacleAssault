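; BP_Third is a Blueprint with a CharacterMovement component that nudges itself back and forth every frame.
; Tick calls the parent, then makes two swept MoveUpdatedComponent calls with opposite one-unit X and Y offsets at the current rotation, netting no displacement unless a sweep is blocked.
; BeginPlay and ActorBeginOverlap are disabled stubs, and the construction script only calls its parent.
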(event EventBeginPlay
  (|CallParentFunction) ; This node is disabled and will not be called.\nDrag off pins to build functionality.
)

(event Collision|EventActorBeginOverlap
  (params (OtherActor :type Actor%20Object%20Reference))
  (|CallParentFunction OtherActor) ; This node is disabled and will not be called.\nDrag off pins to build functionality.
)

(event EventTick
  (params (DeltaSeconds :type Float%20%28single-precision%29))
  (bind _returnvalue (Transformation|GetActorRotation))
  (bind _charactermovement (Variables|Character|GetCharacterMovement))
  (|CallParentFunction DeltaSeconds)
  (Class|MovementComponent|MoveUpdatedComponent _charactermovement "1.000000,1.000000,0.000000" _returnvalue true)
  (Class|MovementComponent|MoveUpdatedComponent _charactermovement "-1.000000,-1.000000,0.000000" _returnvalue true))

(fn ConstructionScript
  (|CallParentFunction))